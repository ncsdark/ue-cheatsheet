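; B_Actor is an Actor Blueprint that serves as an annotated reference sheet of common Blueprint nodes rather than working gameplay.
; Its event graph holds disconnected, commented examples covering flow control, spawning, delays, dispatcher binding, movement, input, tracing, camera, navigation and materials.
; Only the ActorBeginOverlap override is live, forwarding to the parent; the bindable overlap event and Construction Script are empty.
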(event Custom|Bound%20Event
  (params (OverlappedActor :type Actor%20Object%20Reference) (OtherActor :type Actor%20Object%20Reference))
  ;[0.15 0.15 0.15 0.5 60] Event
)

(event Collision|EventActorBeginOverlap
  (params (OtherActor :type Actor%20Object%20Reference))
  ;[0.15 0.15 0.15 0.5 60] Event
  (|CallParentFunction OtherActor))

(fn ConstructionScript)